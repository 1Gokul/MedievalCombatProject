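; Player controller Blueprint that drives the game's UI: HUD overlay, pause menu, inventory menu, and item interact and search prompts.
; It extends parent events, some called from C++, with forward and reverse widget animations and delayed visibility changes.
; Opening the inventory first refreshes item data from class defaults, keeping quantities, then creates the menu.
; Each new prompt clears existing ones and attaches to the HUD canvas at a fixed position.
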(event `self.DisplayHUD`
  (`parent.DisplayHUD`)
  (bind _asmain_player_controller_bp (cast `/Game/Character/MainPlayerController_BP` (`GameplayStatics.GetPlayerController` 0)))
  (bind _ashudoverlay (cast `/Game/HUD/BaseHUD/HUDOverlay` (`MainPlayerController.HUDOverlay` _asmain_player_controller_bp)))
  (`UserWidget.PlayAnimationReverse` _ashudoverlay (`/Game/HUD/BaseHUD/HUDOverlay.HUDAnimation` _ashudoverlay) 6.0 false)
  (`KismetSystemLibrary.Delay` 0.5)
  (`Widget.SetVisibility` _ashudoverlay "Visible"))

(event `self.HideHUD`
  (`parent.HideHUD`)
  (bind _asmain_player_controller_bp (cast `/Game/Character/MainPlayerController_BP` (`GameplayStatics.GetPlayerController` 0)))
  (bind _ashudoverlay (cast `/Game/HUD/BaseHUD/HUDOverlay` (`MainPlayerController.HUDOverlay` _asmain_player_controller_bp)))
  (`UserWidget.PlayAnimationForward` _ashudoverlay (`/Game/HUD/BaseHUD/HUDOverlay.HUDAnimation` _ashudoverlay) 1.0 false))

(event `self.DisplayPauseMenu`
  ;[1 1 1] Pause Menu
  (`parent.DisplayPauseMenu`)
  (bind _aspause_menu (cast `/Game/HUD/PauseMenu/PauseMenu` (`self.PauseMenu`)))
  (`UserWidget.PlayAnimation` _aspause_menu (`/Game/HUD/PauseMenu/PauseMenu.PauseMenuAnimation` _aspause_menu) 0.0 1 "Forward" 1.0 false))

(event `self.RemovePauseMenu`
  ;[1 1 1] Pause Menu
  (`parent.RemovePauseMenu`)
  (bind _aspause_menu (cast `/Game/HUD/PauseMenu/PauseMenu` (`self.PauseMenu`)))
  (`UserWidget.PlayAnimation` _aspause_menu (`/Game/HUD/PauseMenu/PauseMenu.PauseMenuAnimation` _aspause_menu) 0.0 1 "Reverse" 1.0 false)
  (`KismetSystemLibrary.Delay` 0.25)
  (`Widget.SetVisibility` (`self.PauseMenu`) "Hidden"))

(event `self.DisplayInventoryMenu`
  (params (InventoryComponent :type "InventoryComponent Object Reference"))
  ;[1 1 1] Inventory Menu
  (`parent.DisplayInventoryMenu` InventoryComponent)
  (`self.AddDefaultItems` InventoryComponent)
  (bind _returnvalue (`|CreateWidget` "/Game/HUD/InventorySystem/InventoryMenu_WidgetBP.InventoryMenu_WidgetBP_C" null InventoryComponent))
  (`UserWidget.AddToViewport` _returnvalue 0)
  (bind _output_get (set `self.Inventory_Menu` _returnvalue))
  (`UserWidget.PlayAnimation` _output_get (`/Game/HUD/InventorySystem/InventoryMenu_WidgetBP.InventoryMenuBoxAnimation` _returnvalue) 0.0 1 "Forward" 1.0 false)
  (`KismetSystemLibrary.Delay` 0.2))

(event `self.RemoveInventoryMenu`
  (bind _inventory_menu (`self.Inventory_Menu`))
  ;[1 1 1] Inventory Menu
  (`UserWidget.PlayAnimation` _inventory_menu (`/Game/HUD/InventorySystem/InventoryMenu_WidgetBP.InventoryMenuBoxAnimation` _inventory_menu) 0.0 1 "Reverse" 1.0 false)
  (`KismetSystemLibrary.Delay` 0.25)
  (`Widget.RemoveFromParent` (`self.Inventory_Menu`))
  (set `self.Inventory_Menu` null)
  (`parent.RemoveInventoryMenu`))

(event `self.DisplayItemInteractPrompt`
  (params (ItemName :type String) (Weight :type "Float (single-precision)") (Value :type Integer) (InteractText :type Name))
  (`self.RemoveSearchPrompt`) ; Remove existing Search Prompts if any
  (`self.RemoveItemInteractPrompt`)
  (bind _returnvalue (`|CreateWidget` "/Game/HUD/ItemInteractPrompt/ItemInteractPrompt.ItemInteractPrompt_C" null ItemName Weight Value InteractText)) ; Create the Widget
  (set `self.InteractPrompt` _returnvalue)
  (bind _asmain_player_controller_bp (cast `/Game/Character/MainPlayerController_BP` (`GameplayStatics.GetPlayerController` 0)))
  (bind _ashudoverlay (cast `/Game/HUD/BaseHUD/HUDOverlay` (`MainPlayerController.HUDOverlay` _asmain_player_controller_bp)))
  (bind _returnvalue_2 (`CanvasPanel.AddChildToCanvas` (`/Game/HUD/BaseHUD/HUDOverlay.HUDCanvas` _ashudoverlay) (`self.InteractPrompt`))) ; Add the Prompt to the HUD
  (`CanvasPanelSlot.SetAutoSize` _returnvalue_2 true)
  (`CanvasPanelSlot.SetPosition` _returnvalue_2 (760.0 540.0)) ; The Prompt will appear in the center of the screen
  (`parent.DisplayItemInteractPrompt` "" 0.0 0 "None"))

(event `self.RemoveItemInteractPrompt`
  (bind _foundwidgets (`WidgetBlueprintLibrary.GetAllWidgetsOfClass` "/Game/HUD/ItemInteractPrompt/ItemInteractPrompt.ItemInteractPrompt_C" false)) ; Get all existing ItemInteractPrompt Widgets
  (`Widget.RemoveFromParent` _foundwidgets) ; Remove all of them
  (`parent.RemoveItemInteractPrompt`))

(event `self.DisplaySearchPrompt`
  (params (ItemName :type String) (SearchText :type Name))
  (`self.RemoveSearchPrompt`)
  (`self.RemoveItemInteractPrompt`)
  (bind _returnvalue (`|CreateWidget` "/Game/HUD/SearchPrompt/SearchPrompt.SearchPrompt_C" null ItemName SearchText))
  (set `self.SearchPrompt` _returnvalue)
  (bind _asmain_player_controller_bp (cast `/Game/Character/MainPlayerController_BP` (`GameplayStatics.GetPlayerController` 0)))
  (bind _ashudoverlay (cast `/Game/HUD/BaseHUD/HUDOverlay` (`MainPlayerController.HUDOverlay` _asmain_player_controller_bp)))
  (bind _returnvalue_2 (`CanvasPanel.AddChildToCanvas` (`/Game/HUD/BaseHUD/HUDOverlay.HUDCanvas` _ashudoverlay) (`self.SearchPrompt`)))
  (`CanvasPanelSlot.SetAutoSize` _returnvalue_2 true)
  (`CanvasPanelSlot.SetPosition` _returnvalue_2 (760.0 540.0))
  (`parent.DisplaySearchPrompt` "" "None"))

(event `self.RemoveSearchPrompt`
  (bind _foundwidgets (`WidgetBlueprintLibrary.GetAllWidgetsOfClass` "/Game/HUD/SearchPrompt/SearchPrompt.SearchPrompt_C" false))
  (`Widget.RemoveFromParent` _foundwidgets)
  (`parent.RemoveSearchPrompt`))

(fn `AddDefaultItems`
  (params (Inventory :type "InventoryComponent Object Reference"))
  (bind _inventory (`InventoryComponent.Inventory` Inventory))
  (for (_array_element _array_index) _inventory
    (bind (_itemdisplayname _useactiontext _itemdescription _weight _bisstackable _thumbnail _maxstacksize _bisconsumable _bisequippable _value _itemclass) (break `ItemStructure` (break `SlotStructure` _array_element)))
    (if (!= _itemclass null)
      (bind _asitem (castclass `Item` _itemclass))
      (`KismetArrayLibrary.Array_Set` _inventory _array_index (make `SlotStructure` (defaults `Object` _asitem) (`.Quantity` (break `SlotStructure` _array_element)))))))

(fn `UserConstructionScript`)